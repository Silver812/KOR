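; AI controller for the Librarian NPC that runs BT_NPC_Base and drives its blackboard state from AI perception.
; Sounds away from its own pawn trigger Investigating; sight of a non-eliminated player triggers Attacking only while Investigating or Seeking.
; Forgetting the attack target switches to Seeking at that target's location.
; Passive, Attacking and Seeking transitions switch music sections on a tagged AmbientSound through server-to-multicast trigger parameters.
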(event OnPerceptionUpdated(AIPerception)
  (params (UpdatedActors :type Array%20of%20Actor%20Object%20References))
  (for _array_element UpdatedActors
    (Utilities|FlowControl|Sequence
      (:then_0
        (bind _sensed (CallFunction|CanSenseActor _array_element "NewEnumerator1"))
        (if _sensed
          (CallFunction|HandleSensedSight _array_element)))
      (:then_1
        (bind (_sensed_2 _stimulus) (CallFunction|CanSenseActor _array_element "NewEnumerator2"))
        (if _sensed_2
          (CallFunction|HandleSensedSound (.stimuluslocation _stimulus)))))))

(event OnTargetPerceptionForgotten(AIPerception)
  (params (Actor :type Actor%20Object%20Reference))
  (CallFunction|HandleForgottenActor Actor))

(event Custom|ChangeMusic_Server
  (params (Section :type Name) (AudioComponent :type Audio%20Component%20Object%20Reference))
  (CallFunction|ChangeMusicMulticast Section AudioComponent))

(event Custom|ChangeMusic_Multicast
  (params (Section :type Name) (AudioComponent :type Audio%20Component%20Object%20Reference))
  (Class|AudioParameterControllerInterface|SetTriggerParameter AudioComponent Section))

(event EventBeginPlay
  (CallFunction|SetStateasPassive)
  (bind _outactors (Actor|GetAllActorswithTag (Variables|AI|GetMusicTag)))
  (if (Utilities|Array|IsEmpty _outactors)
    (Development|PrintString "No music assigned for the Librarian!" true true "(R=1.000000,G=0.072473,B=0.053819,A=1.000000)")
    (else
      (bind _asambient_sound (Utilities|Casting|CastToAmbientSound (Utilities|Array|Get(acopy) _outactors)))
      (Variables|AI|SetMSSource _asambient_sound))))

(event EventPossess
  (params (PossessedPawn :type Pawn%20Object%20Reference))
  (AI|RunBehaviorTree "/Game/KingOfRecess/Blueprints/AI/BT_NPC_Base.BT_NPC_Base"))

(fn ConstructionScript)

(fn SetStateasPassive
  (AI|Components|Blackboard|SetValueasEnum (Variables|Default|GetBlackboard) (Variables|AI|GetStateKeyName) (Utilities|Enum|LiteralenumE_AIState "NewEnumerator0"))
  (bind _mssource (Variables|AI|GetMSSource)
    (:then
      (CallFunction|ChangeMusicServer "SectionB" (Variables|/Script/Engine.AmbientSound|GetAudioComponent _mssource)))
    (:else)))

(fn CanSenseActor
  (params (Actor :type Actor%20Object%20Reference) (Sense :type E_AISense%20Enum :default "NewEnumerator0"))
  (bind _info (Class|AIPerceptionComponent|GetActorsPerception (Variables|Default|GetAIPerception) Actor))
  (for _array_element (.lastsensedstimuli _info)
    (bind _returnvalue (Class|AIPerceptionSystem|GetSenseClassforStimulus _array_element))
    (if (== _returnvalue (Utilities|Select :Index Sense :Option%200 0 :Option%201 "/Script/AIModule.AISense_Sight" :Option%202 "/Script/AIModule.AISense_Hearing"))
      (return (.bSuccessfullySensed (Utilities|Struct|BreakAIStimulus _array_element)) _array_element))))

(fn HandleSensedSight
  (params (Actor :type Actor%20Object%20Reference))
  (bind _asbp_korcharacter (Utilities|Casting|CastToBP_KORCharacter Actor))
  (if (not (Variables|/Game/KingOfRecess/Blueprints/Game/Characters/KORCharacter/BP_KORCharacter.BP_KORCharacter_C|GetIsEliminated _asbp_korcharacter))
    (bind _state (CallFunction|GetCurrentState))
    (switch Utilities|FlowControl|Switch|SwitchonE_AIState _state
      (:NewEnumerator3
        _)
      (:NewEnumerator5
        _))
    (CallFunction|SetStateasAttacking Actor)))

(fn HandleSensedSound
  (params (Location :type Vector))
  ;[0.1615 0.2045 1] Try to ignore the sounds coming from the librarian moving itself
  (if (> (Math|Vector|Distance(Vector) Location (Transformation|GetActorLocation (Pawn|GetControlledPawn))) 1.5e+02)
    (bind _state (CallFunction|GetCurrentState))
    (switch Utilities|FlowControl|Switch|SwitchonE_AIState _state
      (:NewEnumerator0
        _)
      (:NewEnumerator3
        _)
      (:NewEnumerator5
        _))
    (CallFunction|SetStateasInvestigating Location)))

(fn SetStateasAttacking
  (params (AttackTarget :type Actor%20Object%20Reference))
  (bind _blackboard (Variables|Default|GetBlackboard))
  (Variables|AI|SetAttack%20Target AttackTarget)
  (AI|Components|Blackboard|SetValueasEnum _blackboard (Variables|AI|GetStateKeyName) (Utilities|Enum|LiteralenumE_AIState "NewEnumerator1"))
  (AI|Components|Blackboard|SetValueasObject _blackboard (Variables|AI|GetAttackTargetKeyName) AttackTarget)
  (bind _mssource (Variables|AI|GetMSSource)
    (:then
      (CallFunction|ChangeMusicServer "SectionC" (Variables|/Script/Engine.AmbientSound|GetAudioComponent _mssource)))
    (:else)))

(fn GetCurrentState
  (return (Utilities|Enum|ByteToEnumE_AIState (Class|BlackboardComponent|GetValueasEnum (Variables|Default|GetBlackboard) (Variables|AI|GetStateKeyName)))))

(fn SetStateasInvestigating
  (params (Location :type Vector))
  (bind _blackboard (Variables|Default|GetBlackboard))
  (AI|Components|Blackboard|SetValueasEnum _blackboard (Variables|AI|GetStateKeyName) (Utilities|Enum|LiteralenumE_AIState "NewEnumerator3"))
  (AI|Components|Blackboard|SetValueasVector _blackboard (Variables|AI|GetPointOfInterestKeyName) Location))

(fn HandleForgottenActor
  (params (Actor :type Actor%20Object%20Reference))
  (if (== Actor (Variables|AI|GetAttack%20Target))
    (bind _state (CallFunction|GetCurrentState))
    (switch Utilities|FlowControl|Switch|SwitchonE_AIState _state
      (:NewEnumerator1
        _)
      (:NewEnumerator2
        _)
      (:NewEnumerator3
        _))
    (CallFunction|SetStateasSeeking (Transformation|GetActorLocation (Variables|AI|GetAttack%20Target)))))

(fn HandleLostSight
  (params (Actor :type Actor%20Object%20Reference))
  (if (== Actor (Variables|AI|GetAttack%20Target))
    (bind _state (CallFunction|GetCurrentState))
    (switch Utilities|FlowControl|Switch|SwitchonE_AIState _state
      (:NewEnumerator1
        _)
      (:NewEnumerator2
        _)
      (:NewEnumerator3
        _))
    (CallFunction|SetStateasSeeking (Transformation|GetActorLocation (Variables|AI|GetAttack%20Target)))))

(fn SetStateasSeeking
  (params (Location :type Vector))
  (bind _blackboard (Variables|Default|GetBlackboard))
  (AI|Components|Blackboard|SetValueasEnum _blackboard (Variables|AI|GetStateKeyName) (Utilities|Enum|LiteralenumE_AIState "NewEnumerator5"))
  (AI|Components|Blackboard|SetValueasVector _blackboard (Variables|AI|GetPointOfInterestKeyName) Location)
  (bind _mssource (Variables|AI|GetMSSource)
    (:then
      (CallFunction|ChangeMusicServer "SectionB" (Variables|/Script/Engine.AmbientSound|GetAudioComponent _mssource)))
    (:else)))