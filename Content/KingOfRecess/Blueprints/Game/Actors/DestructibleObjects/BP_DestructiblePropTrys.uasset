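; BP_DestructiblePropTrys is a destructible prop actor that configures its DestructibleObjectComp from data.
; It uses the component's ObjType enum as the row name in DT_DestructibleObjectsData and copies the row into ObjStruct when the types match.
; The lookup runs in both the Construction Script and BeginPlay, and prints an on-screen error if the row is missing.
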(event EventBeginPlay
  (Setter|SetDestructibleObjectData))

(event Collision|EventActorBeginOverlap
  (params (OtherActor :type Actor%20Object%20Reference)))

(event EventTick
  (params (DeltaSeconds :type Float%20%28single-precision%29)))

(fn ConstructionScript
  (Setter|SetDestructibleObjectData))

(fn SetDestructibleObjectData
  (bind _destructibleobjectcomp (Variables|Default|GetDestructibleObjectComp))
  (bind _objtype (Variables|/Script/KOR.ACDestructibleObjectComponent|GetobjType _destructibleobjectcomp))
  (bind _returnvalue (Utilities|GetDataTableRow "/Game/KingOfRecess/Blueprints/Data/DestructibleObjects/DT_DestructibleObjectsData.DT_DestructibleObjectsData" (Utilities|String|StringToName (Utilities|String|EnumtoString _objtype)))
    (:then
      (if (Utilities|Enum|Equal(Enum) (.objType (Utilities|Struct|BreakDestructibleObjectStruct _returnvalue)) _objtype)
        (Variables|/Script/KOR.ACDestructibleObjectComponent|SetObjStruct _destructibleobjectcomp _returnvalue)))
    (:RowNotFound
      (Development|PrintString "DATA TABLE OF DESTRUCTIBLE OBJECT NOT FOUND" true true "(R=0.389583,G=0.040425,B=0.000000,A=1.000000)" 1e+03))))