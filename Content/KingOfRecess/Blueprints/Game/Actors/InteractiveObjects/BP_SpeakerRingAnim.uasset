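; Interactive-object actor that animates a speaker's pitch when play begins, apparently as a ringing shake.
; BeginPlay starts the SpeakerShake timeline, then after a four-second delay calls StopAnim, which plays a second timeline.
; Both timelines drive the Speaker component's relative pitch from their curves, preserving roll and yaw.
; StopAnim does not explicitly stop the shake timeline.
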(event Custom|StopAnim
  (bind _speaker (Variables|Default|GetSpeaker))
  (bind _relativerotation (Variables|/Script/Engine.SceneComponent|GetRelativeRotation _speaker))
  (bind _yrotationaxis (Timeline|Timeline PlayFromStart)
    (:Update
      (Transformation|SetRelativeRotation _speaker (Math|Rotator|MakeRotator (.roll _relativerotation) _yrotationaxis (.yaw _relativerotation)) false false))))

(event Custom|AnimSpeaker
  (bind _speaker (Variables|Default|GetSpeaker))
  (bind _relativerotation (Variables|/Script/Engine.SceneComponent|GetRelativeRotation _speaker))
  (bind _yrotationaxis (Timeline|SpeakerShake PlayFromStart)
    (:Update
      (Transformation|SetRelativeRotation _speaker (Math|Rotator|MakeRotator (.roll _relativerotation) _yrotationaxis (.yaw _relativerotation)) false false))))

(event EventBeginPlay
  (CallFunction|AnimSpeaker)
  (Utilities|FlowControl|Delay 4.0)
  (CallFunction|StopAnim))

(event Collision|EventActorBeginOverlap
  (params (OtherActor :type Actor%20Object%20Reference)))

(event EventTick
  (params (DeltaSeconds :type Float%20%28single-precision%29)))

(fn ConstructionScript)