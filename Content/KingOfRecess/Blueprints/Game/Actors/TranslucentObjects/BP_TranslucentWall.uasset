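; Wall actor that fades translucent as the player character gets close to it along the X axis.
; Construction creates a dynamic material instance on the Wall mesh.
; When Translucent is set, Tick drives its MaterialOpacity from the signed X offset to the cached KORCharacter.
; Opacity scales linearly with distance inside an asymmetric range, longer on the positive X side, and stays opaque outside it.
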(event EventTick
  (params (DeltaSeconds :type Float%20%28single-precision%29))
  (WallBehaviour|TranslucentBehaviour))

(fn ConstructionScript
  (bind _returnvalue (Rendering|Material|CreateDynamicMaterialInstance (Variables|Default|GetWall) 0 "/Game/KingOfRecess/Materials/MI_TranslucentMaterial.MI_TranslucentMaterial" "None" :!class /Script/Engine.PrimitiveComponent))
  (Variables|References|SetMI_TranslucentMaterial _returnvalue))

(fn GetKORPlayer
  (Variables|References|GetKORCharacter
    (:then
      _)
    (:else
      (bind _askorcharacter (Utilities|Casting|CastToKORCharacter (Game|GetPlayerCharacter 0)))
      (Variables|References|SetKORCharacter _askorcharacter)))
  (return (Variables|References|GetKORCharacter)))

(fn XValueDiference
  (Utilities|IsValid (Getter|GetKORPlayer)
    (:Is%20Valid
      (return (- (.x (Transformation|GetWorldLocation (Variables|/Script/Engine.Actor|GetRootComponent (Getter|GetKORPlayer)))) (.x (Transformation|GetWorldLocation (Variables|Default|GetWall))))))
    (:Is%20Not%20Valid
      (return 1e+03))))

(fn XDiferenceAbsoluteValue
  (if (> (Getter|XValueDiference) 0.0)
    (if (< (Getter|XValueDiference) 3.5e+02)
      (return (|(((CurrentXDistance*100)/350)/100) (Getter|XValueDiference)))
      (else
        (return 1.0)))
    (elif (> (Getter|XValueDiference) -1e+02)
      (return (|(((CurrentXDistance*100)/100)/100) (Math|Float|Absolute(Float) (Getter|XValueDiference))))
      (else
        (return 1.0)))))

(fn TranslucentBehaviour
  (if (Variables|WallBehaviour|GetbTranslucent)
    (Rendering|Material|SetScalarParameterValue (Variables|References|GetMI_TranslucentMaterial) "MaterialOpacity" (Getter|XDiferenceAbsoluteValue) :!class /Script/Engine.MaterialInstanceDynamic)))