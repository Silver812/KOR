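; Blackboard actor that serves as a scoreboard, taking over the player's camera and spinning to present the score ranking.
; TurnCamera calls MulticastTurnCamera, which blends the local view to this actor, then plays a Timeline yawing the board 180 degrees.
; A FlipFlop on Finished fills the Top3 and Others texts from the player controller's ScoreManager while flipped, reveals them, then reverses the spin.
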(event Custom|MulticastTurnCamera
  (bind _blackboard (Variables|Default|GetBlackboard))
  (bind _relativerotation (Variables|/Script/Engine.SceneComponent|GetRelativeRotation _blackboard))
  (Game|Player|SetViewTargetwithBlend (Game|GetPlayerController 0) self (Variables|Default|GetBlend%20Time) "VTBlend_Linear" 1.0 false)
  (Utilities|FlowControl|Delay (+ (Variables|Default|GetBlend%20Time) 0.5))
  (bind _alpha (Timeline|Timeline PlayFromStart)
    (:Update
      (Transformation|SetRelativeRotation (Variables|Default|GetBlackboard) (Math|Rotator|MakeRotator (.roll _relativerotation) (.pitch _relativerotation) (* 1.8e+02 _alpha)) false false))
    (:Finished
      (Utilities|FlowControl|FlipFlop
        (:A
          (CallFunction|UpdateScore (Class|ScoreManager|GetScores (Subsystems|GetScoreManager (Game|GetPlayerController 0))))
          (Rendering|SetVisibility (Variables|Default|GetTop3) true false)
          (Utilities|FlowControl|Delay 0.5)
          (Timeline|Timeline ReverseFromEnd))))))

(event Custom|UpdateScore
  (params (ScoreNames :type Array%20of%20Names))
  (Variables|Default|SetTop3Text "")
  (Variables|Default|SetOtherText "")
  (for (_array_element _array_index) ScoreNames
    (if (> _array_index 2)
      (Variables|Default|SetOtherText (Utilities|String|Append (Variables|Default|GetOtherText) (Utilities|String|Append (Utilities|String|ToString(Integer) (+ _array_index 1)) ". " (Utilities|String|ToString(Name) _array_element) " 
")))
      (else
        (Variables|Default|SetTop3Text (Utilities|String|Append (Variables|Default|GetTop3Text) (Utilities|String|Append (Utilities|String|ToString(Integer) (+ _array_index 1)) ". " (Utilities|String|ToString(Name) _array_element) " 
"))))))
  (Rendering|Components|TextRender|SetText (Variables|Default|GetTop3) (Utilities|Text|ToText(String) (Variables|Default|GetTop3Text)))
  (Rendering|Components|TextRender|SetText (Variables|Default|GetOthers) (Utilities|Text|ToText(String) (Variables|Default|GetOtherText))))

(event EventTurnCamera
  (CallFunction|MulticastTurnCamera))

(fn ConstructionScript)