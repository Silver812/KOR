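; Player character for King of Recess, with a floating name widget, physics-driven hands and knockout handling.
; Tick scales animation rate by input acceleration and, on the server, pushes both hands along velocity.
; Jumping while accelerating launches the character in that direction and rolls the mesh through a timeline flip; the wall trace result is unused.
; Elimination disables input, attaches knockout stars, then calls Die on the owning controller after a delay.
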(event Custom|ExecuteDieFunc
  (bind _askor_base_pc (Utilities|Casting|CastToKorBasePC (Components|GetOwner)))
  (Class|KorBasePC|Die _askor_base_pc))

(event Custom|He%20pulsado%20el%20boton
  (Class|PrimitiveComponent|AddTorqueinDegrees (Variables|Default|GetHand_r) (* (Math|Vector|GetUpVector (Variables|Default|GetHand_l)) 2e+02) "None" true))

(event Custom|StopFlip
  (bind _mesh (Variables|Character|GetMesh))
  (bind _relativerotation (Variables|/Script/Engine.SceneComponent|GetRelativeRotation _mesh))
  (bind _relativelocation (Variables|/Script/Engine.SceneComponent|GetRelativeLocation _mesh))
  (bind (_direction _alpha _alpharelativez) (Timeline|Timeline Stop)
    (:Update
      (Transformation|SetRelativeLocationAndRotation _mesh (Math|Vector|MakeVector (.x _relativelocation) (.y _relativelocation) (+ (Variables|Default|GetRelative%20Location%20Z) (* _alpharelativez 5e+01))) (Math|Rotator|MakeRotator (* _alpha 3.6e+02) (.pitch _relativerotation) (.yaw _relativerotation)) false false))))

(event Custom|DoBackflip
  (bind _capsulecomponent (Variables|Default|GetCapsuleComponent))
  (bind _charactermovement (Variables|Character|GetCharacterMovement))
  (bind _returnvalue (Transformation|GetWorldLocation _capsulecomponent))
  (bind _returnvalue_2 (Collision|MultiLineTraceByChannel _returnvalue (+ _returnvalue (* (Math|Vector|Normalize (Math|Vector|GetForwardVector _capsulecomponent)) (Variables|Default|GetDistanceThreshold))) "TraceTypeQuery3" false 0 "None" true "(R=0.676412,G=0.693554,B=1.000000,A=1.000000)"))
  (if (>= (Math|Vector|VectorLength (Pawn|Components|CharacterMovement|GetCurrentAcceleration _charactermovement)) (* (Variables|/Script/Engine.CharacterMovementComponent|GetMaxAcceleration _charactermovement) 0.3))
    (Utilities|FlowControl|Delay 0.1)
    (Character|LaunchCharacter (* (Math|Vector|Normalize (Pawn|Components|CharacterMovement|GetCurrentAcceleration (Variables|Character|GetCharacterMovement))) (Variables|Default|GetLaunchVelocity)) false false)
    (bind _output_get (Variables|Default|SetRelative%20Rotation (Variables|/Script/Engine.SceneComponent|GetRelativeRotation (Variables|Character|GetMesh))))
    (CallFunction|StartFlip "0, 0, 0" _output_get)))

(event Custom|StartFlip
  (params (Axis :type Vector) (InRot :type Rotator))
  (bind _mesh (Variables|Character|GetMesh))
  (bind _relativerotation (Variables|/Script/Engine.SceneComponent|GetRelativeRotation _mesh))
  (bind _relativelocation (Variables|/Script/Engine.SceneComponent|GetRelativeLocation _mesh))
  (Variables|Default|SetRelative%20Location%20Z (.z _relativelocation))
  (bind (_direction _alpha _alpharelativez) (Timeline|Timeline PlayFromStart)
    (:Update
      (Transformation|SetRelativeLocationAndRotation _mesh (Math|Vector|MakeVector (.x _relativelocation) (.y _relativelocation) (+ (Variables|Default|GetRelative%20Location%20Z) (* _alpharelativez 5e+01))) (Math|Rotator|MakeRotator (* _alpha 3.6e+02) (.pitch _relativerotation) (.yaw _relativerotation)) false false))))

(event Custom|SetEliminateState
  (Variables|Default|SetIsEliminated true)
  (Input|DisableInput (CallFunction|GetPCRef))
  (Niagara|SpawnSystemAttached "/Game/KingOfRecess/VFX/Knockout/NS_KnockoutInfinite.NS_KnockoutInfinite" (Variables|Character|GetMesh) "Stars_Socket" "0, 0, 0" "0, 0, 0" "SnapToTarget" true)
  (Utilities|FlowControl|Delay 3.0)
  (CallFunction|ExecuteDieFunc))

(event Custom|ClientTurnCamera
  (Game|Player|SetViewTargetwithBlend (Game|GetPlayerController 0) self 1.0 "VTBlend_Linear" 0.0 false))

(event EventBeginPlay
  (if (Variables|Default|GetHidePlayerName)
    (Development|SetHiddeninGame (Variables|Default|GetPlayerName) true true)
    (else
      (bind _asw_player_name (Utilities|Casting|CastToW_PlayerName (UserInterface|GetWidget (Variables|Default|GetPlayerName))))
      (Utilities|FlowControl|Delay 2.0)
      (bind _askor_base_ps (Utilities|Casting|CastToKorBasePS (Variables|Default|GetPlayerState)))
      (Default|SetText _asw_player_name (Utilities|Text|ToText(Name) (Class|KorBasePS|GetPlayerNameKor _askor_base_ps))))))

(event EventOnJumped
  ;[1 1 1] Intento de backflips
  (CallFunction|DoBackflip))

(event EventTick
  (params (DeltaSeconds :type Float%20%28single-precision%29))
  (Utilities|FlowControl|Sequence
    (:then_0
      (CallFunction|UpdateAnimationScale))
    (:then_1
      (if (Networking|IsServer)
        (Physics|AddImpulse (Variables|Default|GetHand_r) (* (Math|Vector|Normalize (Variables|/Script/Engine.MovementComponent|GetVelocity (Variables|Character|GetCharacterMovement))) (Variables|Default|GetHandImpulse)) "None" false)))))

(event EventTurnCamera
  (CallFunction|ClientTurnCamera))

(fn ConstructionScript)

(fn UpdateAnimationScale
  (Variables|/Script/Engine.SkeletalMeshComponent|SetGlobalAnimRateScale (Variables|Character|GetMesh) (+ (/ (Math|Vector|VectorLength (Pawn|Components|CharacterMovement|GetCurrentAcceleration (Variables|Character|GetCharacterMovement))) (Class|CharacterMovementComponent|GetMaxAcceleration (Variables|Character|GetCharacterMovement))) 0.3)))

(fn GetPCRef
  (Variables|Default|GetPCRef
    (:then
      _)
    (:else
      (bind _asplayer_controller (Utilities|Casting|CastToPlayerController (Pawn|GetController)))
      (Variables|Default|SetPCRef _asplayer_controller)))
  (return (Variables|Default|GetPCRef)))