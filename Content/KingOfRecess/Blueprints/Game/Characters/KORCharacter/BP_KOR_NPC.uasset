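; BP_KOR_NPC is an AI-controlled character that patrols and catches players in King of Recess.
; On BeginPlay it finds its patrol route by actor tag, a workaround for a bugged instance-editable variable.
; On the server, a CatchRange overlap with the attack target while Attacking eliminates that player, sets the AI passive and passes the player's name to KorScorer.
; Helpers lazily cache the AI controller and map speed modes to walk speed.
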(event OnComponentBeginOverlap(CatchRange)
  (params (OverlappedComponent :type Primitive%20Component%20Object%20Reference) (OtherActor :type Actor%20Object%20Reference) (OtherComp :type Primitive%20Component%20Object%20Reference) (OtherBodyIndex :type Integer) (bFromSweep :type Boolean) (SweepResult :type Hit%20Result%20Structure%20%28by%20ref%29))
  (Networking|SwitchHasAuthority
    (:Authority
      (if (not (== self OtherActor))
        (bind _state (Default|GetCurrentState (CallFunction|GetControllerRef)))
        (switch Utilities|FlowControl|Switch|SwitchonE_AIState _state
          (:NewEnumerator1
            (if (== OtherActor (Variables|/Game/KingOfRecess/Blueprints/AI/Blueprints/BP_KorAIController.BP_KorAIController_C|GetAttack%20Target (CallFunction|GetControllerRef)))
              (bind _asbp_korcharacter (Utilities|Casting|CastToBP_KORCharacter OtherActor))
              (if (not (Variables|/Game/KingOfRecess/Blueprints/Game/Characters/KORCharacter/BP_KORCharacter.BP_KORCharacter_C|GetIsEliminated _asbp_korcharacter))
                (Default|SetStateasPassive (CallFunction|GetControllerRef))
                (Default|SetEliminateState _asbp_korcharacter)
                (bind _askor_base_ps (Utilities|Casting|CastToKorBasePS (Variables|/Script/Engine.Pawn|GetPlayerState _asbp_korcharacter)))
                (Class|KorScorer|PlayerScored (Actor|GetComponentbyClass (Game|GetGameState) "/Script/KOR.KorScorer") (Class|KorBasePS|GetPlayerNameKor _askor_base_ps))))))))))

(event EventBeginPlay
  (|CallParentFunction)
  (CallFunction|InitPatrolRoute))

(fn ConstructionScript
  (|CallParentFunction))

(fn GetControllerRef
  (Variables|IAData|GetAIPCRef
    (:then
      _)
    (:else
      (bind _asbp_kor_aicontroller (Utilities|Casting|CastToBP_KorAIController (AI|GetAIController self)))
      (Variables|IAData|SetAIPCRef _asbp_kor_aicontroller)))
  (return (Variables|IAData|GetAIPCRef)))

(fn InitPatrolRoute
  ;[1 0.2232 0] Instance editable on the Patrol Route variable is bugged
  (bind _outactors (Actor|GetAllActorswithTag (Variables|IAData|GetRouteTag)))
  (if (Utilities|Array|IsEmpty _outactors)
    (Development|PrintString "No patrol route assigned for the AI!" true true "(R=1.000000,G=0.072473,B=0.053819,A=1.000000)")
    (else
      (bind _asbp_patrol_route (Utilities|Casting|CastToBP_PatrolRoute (Utilities|Array|Get(acopy) _outactors)))
      (Variables|IAData|SetPatrolRoute _asbp_patrol_route))))

(fn GetPatrolRoute
  (return (Variables|IAData|GetPatrolRoute)))

(fn SetMovementSpeed
  (params (SpeedMode :type E_AIMovementSpeed%20Enum :default "NewEnumerator0"))
  (bind _output_get (Variables|/Script/Engine.CharacterMovementComponent|SetMaxWalkSpeed (Variables|Character|GetCharacterMovement) (Utilities|Select :Index SpeedMode :NewEnumerator0 0.0 :NewEnumerator1 2e+02 :NewEnumerator2 3e+02 :NewEnumerator3 4.5e+02)))
  (return _output_get))