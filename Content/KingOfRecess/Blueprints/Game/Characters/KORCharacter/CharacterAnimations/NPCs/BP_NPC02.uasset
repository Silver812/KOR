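; BP_NPC02 is an NPC actor in King of Recess that animates its body and feet procedurally with timelines.
; On BeginPlay it starts three timelines, one for the body and one for each foot.
; Each timeline drives the roll of its component's relative rotation, keeping pitch and yaw, to shake the body and the left and right foot pivots.
; Tick, overlap and construction logic are empty.
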(event Custom|BodyShakeAnim
  (bind _body (Variables|Default|GetBody))
  (bind _relativerotation (Variables|/Script/Engine.SceneComponent|GetRelativeRotation _body))
  (bind _rotationxaxis (Timeline|BodyShake PlayFromStart)
    (:Update
      (Transformation|SetRelativeRotation _body (Math|Rotator|MakeRotator _rotationxaxis (.pitch _relativerotation) (.yaw _relativerotation)) false false))))

(event Custom|RightFootShake
  (bind _footscenerotator_right (Variables|Default|GetFootSceneRotator_Right))
  (bind _relativerotation (Variables|/Script/Engine.SceneComponent|GetRelativeRotation _footscenerotator_right))
  (bind _rotatorxaxis (Timeline|RightFootAnim PlayFromStart)
    (:Update
      (Transformation|SetRelativeRotation _footscenerotator_right (Math|Rotator|MakeRotator _rotatorxaxis (.pitch _relativerotation) (.yaw _relativerotation)) false false))))

(event Custom|LeftFootShake
  (bind _footscenerotator_left (Variables|Default|GetFootSceneRotator_Left))
  (bind _relativerotation (Variables|/Script/Engine.SceneComponent|GetRelativeRotation _footscenerotator_left))
  (bind _rotatorxaxis (Timeline|LeftFootAnim PlayFromStart)
    (:Update
      (Transformation|SetRelativeRotation _footscenerotator_left (Math|Rotator|MakeRotator _rotatorxaxis (.pitch _relativerotation) (.yaw _relativerotation)) false false))))

(event EventBeginPlay
  (CallFunction|BodyShakeAnim)
  (CallFunction|RightFootShake)
  (CallFunction|LeftFootShake))

(event Collision|EventActorBeginOverlap
  (params (OtherActor :type Actor%20Object%20Reference)))

(event EventTick
  (params (DeltaSeconds :type Float%20%28single-precision%29)))

(fn ConstructionScript)