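; BP_NPC12 is a King of Recess NPC built from separate body-part components and animated procedurally with timelines.
; On BeginPlay it randomizes clothing and skin materials, then plays left-hand and body roll shakes plus a vertical right-hand motion.
; Each tick, if LookAtKorCharacter is set, the head turns toward the player controller's focal location with a yaw offset.
; Foot, right-hand shake and StrangerAnim events are defined but not triggered here.
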(event Custom|RightFootShake
  (bind _rightfoot_bone (Variables|Default|GetRightFoot_bone))
  (bind _relativerotation (Variables|/Script/Engine.SceneComponent|GetRelativeRotation _rightfoot_bone))
  (bind _rotatorxaxis (Timeline|RightFootAnim PlayFromStart)
    (:Update
      (Transformation|SetRelativeRotation _rightfoot_bone (Math|Rotator|MakeRotator _rotatorxaxis (.pitch _relativerotation) (.yaw _relativerotation)) false false))))

(event Custom|LeftFootShake
  (bind _leftfoot_bone (Variables|Default|GetLeftFoot_bone))
  (bind _relativerotation (Variables|/Script/Engine.SceneComponent|GetRelativeRotation _leftfoot_bone))
  (bind _rotatorxaxis (Timeline|LeftFootAnim PlayFromStart)
    (:Update
      (Transformation|SetRelativeRotation _leftfoot_bone (Math|Rotator|MakeRotator _rotatorxaxis (.pitch _relativerotation) (.yaw _relativerotation)) false false))))

(event Custom|RightHandShake
  (bind _righthand_bone (Variables|Default|GetRightHand_Bone))
  (bind _relativerotation (Variables|/Script/Engine.SceneComponent|GetRelativeRotation _righthand_bone))
  (bind _rotatorxaxis (Timeline|RightHandAnim PlayFromStart)
    (:Update
      (Transformation|SetRelativeRotation _righthand_bone (Math|Rotator|MakeRotator _rotatorxaxis (.pitch _relativerotation) (.yaw _relativerotation)) false false))))

(event Custom|LeftHandShake
  (bind _lefthandbone (Variables|Default|GetLeftHandBone))
  (bind _relativerotation (Variables|/Script/Engine.SceneComponent|GetRelativeRotation _lefthandbone))
  (bind _rotatorxaxis (Timeline|LeftHAndAnim PlayFromStart)
    (:Update
      (Transformation|SetRelativeRotation _lefthandbone (Math|Rotator|MakeRotator _rotatorxaxis (.pitch _relativerotation) (.yaw _relativerotation)) false false))))

(event Custom|BodyShake
  (bind _body (Variables|Default|GetBody))
  (bind _relativerotation (Variables|/Script/Engine.SceneComponent|GetRelativeRotation _body))
  (bind _rotatorxaxis (Timeline|Timeline PlayFromStart)
    (:Update
      (Transformation|SetRelativeRotation _body (Math|Rotator|MakeRotator _rotatorxaxis (.pitch _relativerotation) (.yaw _relativerotation)) false false))))

(event Custom|StrangerAnim
  (bind _character (Variables|Default|GetCharacter))
  (bind _relativerotation (Variables|/Script/Engine.SceneComponent|GetRelativeRotation _character))
  (bind _rotatoryaxis (Timeline|WhoisHe PlayFromStart)
    (:Update
      (Transformation|SetRelativeRotation _character (Math|Rotator|MakeRotator (.roll _relativerotation) _rotatoryaxis (.yaw _relativerotation)) false false))))

(event Custom|GoDownAnim
  (bind _righthand_bone (Variables|Default|GetRightHand_Bone))
  (bind _relativelocation (Variables|/Script/Engine.SceneComponent|GetRelativeLocation _righthand_bone))
  (bind _positionzaxis (Timeline|GoDown_anim PlayFromStart)
    (:Update
      (Transformation|SetRelativeLocation _righthand_bone (Math|Vector|MakeVector (.x _relativelocation) (.y _relativelocation) _positionzaxis) false false))))

(event EventBeginPlay
  (Setter|SetRandomColor)
  (Setter|SetRandomSkin)
  (CallFunction|LeftHandShake)
  (CallFunction|BodyShake)
  (CallFunction|GoDownAnim))

(event Collision|EventActorBeginOverlap
  (params (OtherActor :type Actor%20Object%20Reference)))

(event EventTick
  (params (DeltaSeconds :type Float%20%28single-precision%29))
  (Animations|HeadLookatCharacter))

(fn ConstructionScript)

(fn HeadLookatCharacter
  (bind _returnvalue (Game|GetPlayerController 0))
  (bind _head_bone (Variables|Default|GetHead_Bone))
  (bind _returnvalue_2 (Transformation|GetWorldLocation _head_bone))
  (bind _returnvalue_3 (Class|PlayerController|GetFocalLocation _returnvalue))
  (bind _returnvalue_4 (Math|Rotator|FindLookatRotation _returnvalue_2 _returnvalue_3))
  (if (Variables|NPCBehaviour|GetLookAtKorCharacter)
    (Transformation|SetWorldRotation _head_bone (Math|Rotator|MakeRotator (.roll _returnvalue_4) (.pitch _returnvalue_4) (- (.yaw _returnvalue_4) 9e+01)) false false)))

(fn SetRandomColor
  (bind _clothesmaterialslists (Variables|NPCBehaviour|GetClothesMaterialsLists))
  (bind _output_get (Variables|NPCBehaviour|SetCurrentClotheMat (Utilities|Array|Get(acopy) _clothesmaterialslists (Math|Random|RandomIntegerinRange 0 (- (Utilities|Array|Length _clothesmaterialslists) 1)))))
  (Utilities|IsValid _output_get
    (:Is%20Valid
      (Rendering|Material|SetMaterial (Variables|Default|GetBody) 0 (Variables|NPCBehaviour|GetCurrentClotheMat))
      (Rendering|Material|SetMaterial (Variables|Default|GetLeftFoot) 0 (Variables|NPCBehaviour|GetCurrentClotheMat))
      (Rendering|Material|SetMaterial (Variables|Default|GetRightFoot) 0 (Variables|NPCBehaviour|GetCurrentClotheMat))
      (Rendering|Material|SetMaterial (Variables|Default|GetHead) 1 (Variables|NPCBehaviour|GetCurrentClotheMat))
      (Rendering|Material|SetMaterial (Variables|Default|GetLeftHand) 0 (Variables|NPCBehaviour|GetCurrentClotheMat))
      (Rendering|Material|SetMaterial (Variables|Default|GetRightHand) 0 (Variables|NPCBehaviour|GetCurrentClotheMat)))))

(fn SetRandomSkin
  (bind _skinmaterialslists (Variables|NPCBehaviour|GetSkinMaterialsLists))
  (bind _output_get (Variables|NPCBehaviour|SetCurrentSkinMat (Utilities|Array|Get(acopy) _skinmaterialslists (Math|Random|RandomIntegerinRange 0 (- (Utilities|Array|Length _skinmaterialslists) 1)))))
  (Utilities|IsValid _output_get
    (:Is%20Valid
      (Rendering|Material|SetMaterial (Variables|Default|GetHead) 0 (Variables|NPCBehaviour|GetCurrentSkinMat)))))