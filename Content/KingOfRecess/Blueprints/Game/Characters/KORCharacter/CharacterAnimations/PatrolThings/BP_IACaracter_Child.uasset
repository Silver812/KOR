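; AI child character that wanders between BP_PatrolPoint actors in the main menu and lobby, with randomized clothing and skin materials.
; BeginPlay randomizes materials and gathers patrol points by map selection: all for Main Menu, only those of a matching type for Lobby.
; Main Menu starts with a move to a random X position, flagged in a comment as aborting.
; GoToRandomPatrolPoint chains AIMoveTo calls on success, retrying recursively when no valid point returns.
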(event Custom|GoToRandomPatrolPoint
  (bind _patrolpoint (Getter|GetRandomLocation))
  ;[0.8632 0.305 0.04817] Random PatrolPoint
  (Variables|IABehaviour|SetIAStates "NewEnumerator1")
  (Utilities|IsValid _patrolpoint
    (:Is%20Valid
      (AI|AIMoveTo self (Transformation|GetWorldLocation (Variables|/Game/KingOfRecess/Blueprints/Game/Characters/KORCharacter/CharacterAnimations/PatrolThings/BP_PatrolPoint.BP_PatrolPoint_C|GetCylinder _patrolpoint)) 0 5.0 false
        (:OnSuccess
          (Variables|IABehaviour|SetIAStates "NewEnumerator0")
          (CallFunction|GotoRandomPatrolPoint))))
    (:Is%20Not%20Valid
      (CallFunction|GotoRandomPatrolPoint))))

(event Custom|MainMenuPatrolBehaviour
  ;[0 0.7889 1] MainMenuBehaviour
  (Variables|IABehaviour|SetIAStates "NewEnumerator1")
  ;;[1 0.04432 0 0.5] IT'S ABORTING HERE
  (AI|AIMoveTo self (Math|Vector|MakeVector (Math|Random|RandomFloatinRange -1e+03 0.0) 0.0 0.0) 0 5.0 false
    (:OnSuccess
      (CallFunction|GotoRandomPatrolPoint))
    (:OnFail
      (Development|PrintString "AIMoveTo failed..." true true "(R=1.000000,G=0.058218,B=0.000000,A=1.000000)"))))

(event EventBeginPlay
  (|CallParentFunction)
  (Setter|SetClothesColor)
  (Setter|SetRandomSkinColor)
  (Setter|SetPatrolPointsArray)
  (switch Utilities|FlowControl|Switch|SwitchonE_TypeOfPatrol (Variables|IABehaviour|GetIAMapSelection)
    (:NewEnumerator0
      (CallFunction|MainMenuPatrolBehaviour))
    (:NewEnumerator1
      (CallFunction|GotoRandomPatrolPoint))))

(event Collision|EventActorBeginOverlap
  (params (OtherActor :type Actor%20Object%20Reference))
  (|CallParentFunction OtherActor) ; This node is disabled and will not be called.\nDrag off pins to build functionality.
)

(event EventTick
  (params (DeltaSeconds :type Float%20%28single-precision%29))
  (|CallParentFunction DeltaSeconds))

(fn ConstructionScript
  (|CallParentFunction))

(fn SetPatrolPointsArray
  (switch Utilities|FlowControl|Switch|SwitchonE_TypeOfPatrol (Variables|IABehaviour|GetIAMapSelection)
    (:NewEnumerator0
      (bind _outactors (Actor|GetAllActorsOfClass "/Game/KingOfRecess/Blueprints/Game/Characters/KORCharacter/CharacterAnimations/PatrolThings/BP_PatrolPoint.BP_PatrolPoint_C"))
      (for _array_element _outactors
        (Utilities|Array|Add (Variables|IABehaviour|GetPatrolPoints) _array_element)))
    (:NewEnumerator1
      (bind _outactors_2 (Actor|GetAllActorsOfClass "/Game/KingOfRecess/Blueprints/Game/Characters/KORCharacter/CharacterAnimations/PatrolThings/BP_PatrolPoint.BP_PatrolPoint_C"))
      (for _array_element_2 _outactors_2
        (if (Utilities|Enum|Equal(Enum) (Variables|/Game/KingOfRecess/Blueprints/Game/Characters/KORCharacter/CharacterAnimations/PatrolThings/BP_PatrolPoint.BP_PatrolPoint_C|GetTypeOfPatrolPoint _array_element_2) (Variables|IABehaviour|GetPatrollPointToGo))
          (Utilities|Array|Add (Variables|IABehaviour|GetPatrolPoints) _array_element_2))))))

(fn GetRandomLocation
  (bind _patrolpoints (Variables|IABehaviour|GetPatrolPoints))
  (bind _returnvalue (Utilities|Array|Length _patrolpoints))
  (bind _returnvalue_2 (- _returnvalue 1))
  (bind _returnvalue_3 (Math|Random|RandomIntegerinRange 0 _returnvalue_2))
  (bind _output_get (Variables|IABehaviour|SetPatrolPointSelected _returnvalue_3))
  (if (!= _output_get _returnvalue_3)
    (for (_array_element _array_index) _patrolpoints
      (if (== _array_index (Variables|IABehaviour|GetPatrolPointSelected))
        (return _array_element)))))

(fn SetClothesColor
  (bind _clothesmaterialslists (Variables|SkinBehaviour|GetClothesMaterialsLists))
  (bind _output_get (Variables|SkinBehaviour|SetCurrentClotheMat (Utilities|Array|Get(acopy) _clothesmaterialslists (Math|Random|RandomIntegerinRange 0 (- (Utilities|Array|Length _clothesmaterialslists) 1)))))
  (Utilities|IsValid _output_get
    (:Is%20Valid
      (Rendering|Material|SetMaterial (Variables|Character|GetMesh) 6 (Variables|SkinBehaviour|GetCurrentClotheMat))
      (Rendering|Material|SetMaterial (Variables|Character|GetMesh) 2 (Variables|SkinBehaviour|GetCurrentClotheMat)))))

(fn SetRandomSkinColor
  (bind _skinmaterialslists (Variables|SkinBehaviour|GetSkinMaterialsLists))
  (bind _output_get (Variables|SkinBehaviour|SetCurrentSkinMat (Utilities|Array|Get(acopy) _skinmaterialslists (Math|Random|RandomIntegerinRange 0 (- (Utilities|Array|Length _skinmaterialslists) 1)))))
  (Utilities|IsValid _output_get
    (:Is%20Valid
      (Rendering|Material|SetMaterial (Variables|Character|GetMesh) 0 (Variables|SkinBehaviour|GetCurrentSkinMat)))))