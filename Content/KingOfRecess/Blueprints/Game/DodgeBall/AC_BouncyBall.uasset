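; Actor component for the dodgeball mode that simulates bounciness on the primitive component passed in through SetBounciness.
; Each Tick it line-traces far ahead along that component's velocity, with debug drawing.
; While the trace hits, it draws the reflected direction and adds a velocity-change impulse along it scaled by Bounciness, without waiting for contact.
; Linear damping adjustments are present but disconnected.
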(event Custom|SetBounciness
  (params (NewParam :type Static%20Mesh%20Component%20Object%20Reference)))

(event EventTick
  (params (DeltaSeconds :type Float%20%28single-precision%29))
  (bind (_outhit _returnvalue) (Collision|LineTraceByChannel (Transformation|GetWorldLocation (stale Custom|SetBounciness NewParam)) (+ (Transformation|GetWorldLocation (stale Custom|SetBounciness NewParam)) (* (Transformation|GetComponentVelocity (stale Custom|SetBounciness NewParam)) 2000)) "TraceTypeQuery1" false 0 "ForOneFrame"))
  (if _returnvalue
    (Collision|LineTraceByChannel (.Location (Collision|BreakHitResult _outhit)) (+ (.Location (Collision|BreakHitResult _outhit)) (* (Math|Vector|GetReflectionVector (Math|Vector|GetUnitDirection(Vector) (.TraceStart (Collision|BreakHitResult _outhit)) (.TraceEnd (Collision|BreakHitResult _outhit))) (.Normal (Collision|BreakHitResult _outhit))) 2e+02)) "TraceTypeQuery1" false (Utilities|Array|MakeArray (.HitActor (Collision|BreakHitResult _outhit))) "ForOneFrame")
    (if true
      (Physics|AddImpulse (stale Custom|SetBounciness NewParam) (* (Math|Vector|GetReflectionVector (Math|Vector|GetUnitDirection(Vector) (.TraceStart (Collision|BreakHitResult _outhit)) (.TraceEnd (Collision|BreakHitResult _outhit))) (.Normal (Collision|BreakHitResult _outhit))) (Variables|Default|GetBounciness)) "None" true))))