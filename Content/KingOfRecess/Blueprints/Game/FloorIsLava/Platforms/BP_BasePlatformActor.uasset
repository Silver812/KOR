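; Base platform actor for the Floor Is Lava game that animates its mesh floating up, trembling and sinking through timelines.
; StartFloat raises the mesh from an initial depth, while Sink trembles it for a delay before lowering it, optionally destroying the actor afterwards.
; Afloat stops the tremble, closes a gate to cancel any pending sink and reverses the sink timeline.
; Tremble direction is the cross product of camera and actor forward vectors.
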(event Custom|StartTremble
  (bind _staticmesh (Variables|Default|GetStaticMesh))
  (bind _alpha (Timeline|Tremble Play)
    (:Update
      (Transformation|SetRelativeLocation _staticmesh (+ (Variables|/Script/Engine.SceneComponent|GetRelativeLocation _staticmesh) (* (Math|Vector|CrossProduct (Math|Vector|GetForwardVector (Camera|GetCameraRotation (Variables|/Script/Engine.PlayerController|GetPlayerCameraManager (Game|GetPlayerController 0)))) (Math|Vector|GetForwardVector (Transformation|GetActorRotation))) _alpha (Variables|Default|GetTrembleOffset))) false false))))

(event Custom|StopTremble
  (bind _staticmesh (Variables|Default|GetStaticMesh))
  (bind _alpha (Timeline|Tremble Stop)
    (:Update
      (Transformation|SetRelativeLocation _staticmesh (+ (Variables|/Script/Engine.SceneComponent|GetRelativeLocation _staticmesh) (* (Math|Vector|CrossProduct (Math|Vector|GetForwardVector (Camera|GetCameraRotation (Variables|/Script/Engine.PlayerController|GetPlayerCameraManager (Game|GetPlayerController 0)))) (Math|Vector|GetForwardVector (Transformation|GetActorRotation))) _alpha (Variables|Default|GetTrembleOffset))) false false))))

(event Custom|StartFloat
  (bind _initialdepth (Variables|Default|GetInitialDepth))
  (bind _alpha (Timeline|InitialFloat PlayFromStart)
    (:Update
      (Transformation|SetRelativeLocation (Variables|Default|GetStaticMesh) (+ (* (Math|Vector|MakeVector 0.0 0.0 1.0) _alpha _initialdepth) (Math|Vector|MakeVector 0.0 0.0 (+ (* _initialdepth -1.0) (Variables|Default|GetBuoyancyOffset)))) false false))))

(event Custom|Sink
  (params (Should%20Terminate? :type Boolean))
  (bind _staticmesh (Variables|Default|GetStaticMesh))
  (bind _relativelocation (Variables|/Script/Engine.SceneComponent|GetRelativeLocation _staticmesh))
  (CallFunction|OpenGate)
  (Variables|Default|SetRelativeSinkingOffset (Variables|/Script/Engine.SceneComponent|GetRelativeLocation (Variables|Default|GetStaticMesh)))
  (CallFunction|StartTremble)
  (Utilities|FlowControl|Delay (Variables|Default|GetTrembleDuration))
  (Utilities|FlowControl|Gate true
    (:Exit
      (bind _alpha (Timeline|SinkTimeline PlayFromStart)
        (:Update
          (Transformation|SetRelativeLocation (Variables|Default|GetStaticMesh) (+ (Math|Vector|MakeVector (.x _relativelocation) (.y _relativelocation) (.z (Variables|Default|GetRelativeSinkingOffset))) (* "0.000000,0.000000,1.000000" _alpha (Variables|Default|GetSinkingDistance))) false false))
        (:Finished
          (if Should%20Terminate?
            (Actor|DestroyActor)))))))

(event Custom|Afloat
  (bind _staticmesh (Variables|Default|GetStaticMesh))
  (bind _relativelocation (Variables|/Script/Engine.SceneComponent|GetRelativeLocation _staticmesh))
  (CallFunction|StopTremble)
  (CallFunction|CloseGate)
  (bind _alpha (Timeline|SinkTimeline Reverse)
    (:Update
      (Transformation|SetRelativeLocation (Variables|Default|GetStaticMesh) (+ (Math|Vector|MakeVector (.x _relativelocation) (.y _relativelocation) (.z (Variables|Default|GetRelativeSinkingOffset))) (* "0.000000,0.000000,1.000000" _alpha (Variables|Default|GetSinkingDistance))) false false))
    (:Finished
      (if (stale Custom|Sink Should%20Terminate?)
        (Actor|DestroyActor)))))

(event Custom|OpenGate
  (bind _staticmesh (Variables|Default|GetStaticMesh))
  (bind _relativelocation (Variables|/Script/Engine.SceneComponent|GetRelativeLocation _staticmesh))
  (Utilities|FlowControl|Gate true) ; enters at Open
)

(event Custom|CloseGate
  (bind _staticmesh (Variables|Default|GetStaticMesh))
  (bind _relativelocation (Variables|/Script/Engine.SceneComponent|GetRelativeLocation _staticmesh))
  (Utilities|FlowControl|Gate true) ; enters at Close
)

(fn ConstructionScript)