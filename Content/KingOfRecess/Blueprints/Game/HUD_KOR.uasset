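; HUD for King of Recess that manages the screen widgets around a library minigame.
; Base UI goes through PushWidget, while helper functions create and remove single-instance loading, blackout and fade widgets, though fades are only ever added.
; WidgetBehaviour either shows a timed loading screen with a tutorial popup before the minigame widget or opens it directly, then clears the blackout.
; Its call in the event graph is disconnected.
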(event Custom|InitializeBaseUI
  (params (UIClass :type User%20Widget%20Class%20Reference) (InputMode :type EInputMode%20Enum :default "UI"))
  (Class|KORBaseHUD|PushWidget UIClass InputMode))

(event Custom|CloseTransitionMenuByTime
  (params (Duration :type Float%20%28single-precision%29))
  ;[0.06301 0.003347 0.003035] Close Transition Menu By Time
  (Utilities|FlowControl|Delay Duration)
  (HUDBehaviour|TransitionMenu|CloseTransitionMenu)
  (HUDBehaviour|Minigame|OpenMiniGameMenu))

(event EventBeginPlay)

(fn ConstructionScript)

(fn OpenTransitionMenu
  (params (TutorialPopUp :type E_TutorialPopUp%20Enum :default "NewEnumerator0"))
  (Variables|Getter|GetWGLoadingScreen_Ref
    (:then)
    (:else
      (bind _returnvalue (UserInterface|CreateWidget "/Game/KingOfRecess/Blueprints/UI/LoadingScreen/WG_LoadingScreen.WG_LoadingScreen_C"))
      (bind _output_get (Variables|Getter|SetWGLoadingScreen_Ref _returnvalue))
      (Variables|/Game/KingOfRecess/Blueprints/UI/LoadingScreen/WG_LoadingScreen.WG_LoadingScreen_C|SetTutorialPopUp _output_get TutorialPopUp)
      (UserInterface|Viewport|AddtoViewport _output_get 0))))

(fn CloseTransitionMenu
  (bind _wgloadingscreen_ref (Variables|Getter|GetWGLoadingScreen_Ref)
    (:then
      (Widget|RemovefromParent _wgloadingscreen_ref)
      (Variables|Getter|SetWGLoadingScreen_Ref 0))
    (:else)))

(fn OpenMiniGameMenu
  (Variables|Getter|GetLibraryWG_ref
    (:then)
    (:else
      (bind _returnvalue (UserInterface|CreateWidget "/Game/KingOfRecess/Blueprints/UI/InGameUI/Library/WG_Library.WG_Library_C"))
      (bind _output_get (Variables|Getter|SetLibraryWG_ref _returnvalue))
      (Default|SetMinigameMaxTime _output_get 1.8e+02)
      (UserInterface|Viewport|AddtoViewport _returnvalue 0))))

(fn WidgetBehaviour
  (if (Variables|HUDBehaviour|GetbActiveTransitionScreen)
    (HUDBehaviour|TransitionMenu|OpenTransitionMenu "NewEnumerator0")
    (HUDBehaviour|Blackout|CloseBlackOutWG)
    (CallFunction|CloseTransitionMenubyTime 13.0)
    (else
      (HUDBehaviour|Minigame|OpenMiniGameMenu)
      (HUDBehaviour|Blackout|CloseBlackOutWG))))

(fn OpenBlackOutWG
  (Variables|Getter|GetBlackOut_Ref
    (:then)
    (:else
      (bind _returnvalue (UserInterface|CreateWidget "/Game/KingOfRecess/Blueprints/UI/LoadingScreen/WG_BlackOutWG.WG_BlackOutWG_C"))
      (bind _output_get (Variables|Getter|SetBlackOut_Ref _returnvalue))
      (UserInterface|Viewport|AddtoViewport _output_get 0))))

(fn CloseBlackOutWG
  (bind _blackout_ref (Variables|Getter|GetBlackOut_Ref)
    (:then
      (Widget|RemovefromParent _blackout_ref)
      (Variables|Getter|SetBlackOut_Ref 0))
    (:else)))

(fn FadeOut
  (Variables|Default|GetFadeOutRef
    (:then)
    (:else
      (bind _returnvalue (UserInterface|CreateWidget "/Game/KingOfRecess/Blueprints/UI/LoadingScreen/WG_FadeOutWg.WG_FadeOutWg_C"))
      (bind _output_get (Variables|Default|SetFadeOutRef _returnvalue))
      (UserInterface|Viewport|AddtoViewport _output_get 0))))

(fn Fadein
  (Variables|Default|GetFadeInRef
    (:then)
    (:else
      (bind _returnvalue (UserInterface|CreateWidget "/Game/KingOfRecess/Blueprints/UI/LoadingScreen/WG_FadeInWg.WG_FadeInWg_C"))
      (bind _output_get (Variables|Default|SetFadeInRef _returnvalue))
      (UserInterface|Viewport|AddtoViewport _output_get 0))))