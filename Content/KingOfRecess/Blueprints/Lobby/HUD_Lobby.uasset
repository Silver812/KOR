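; HUD Blueprint for the King of Recess lobby that puts the loading screen and fade-in/fade-out transition widgets on screen.
; Each open function creates its widget, caches the reference and adds it to the viewport, skipping all of this while that reference is still valid.
; The loading screen also receives a TutorialPopUp value from the caller before it is displayed.
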(fn ConstructionScript)

(fn OpenLoadingScreen
  (params (TutorialPopUp :type E_TutorialPopUp%20Enum :default "NewEnumerator0"))
  (Variables|WidgetReferences|GetWGLoadingScreen_Ref
    (:then)
    (:else
      (bind _returnvalue (UserInterface|CreateWidget "/Game/KingOfRecess/Blueprints/UI/LoadingScreen/WG_LoadingScreen.WG_LoadingScreen_C"))
      (bind _output_get (Variables|WidgetReferences|SetWGLoadingScreen_Ref _returnvalue))
      (Variables|/Game/KingOfRecess/Blueprints/UI/LoadingScreen/WG_LoadingScreen.WG_LoadingScreen_C|SetTutorialPopUp _output_get TutorialPopUp)
      (UserInterface|Viewport|AddtoViewport _output_get 0))))

(fn OpenFadein
  (Variables|Default|GetFadeInRef
    (:then)
    (:else
      (bind _returnvalue (UserInterface|CreateWidget "/Game/KingOfRecess/Blueprints/UI/LoadingScreen/WG_FadeInWg.WG_FadeInWg_C"))
      (bind _output_get (Variables|Default|SetFadeInRef _returnvalue))
      (UserInterface|Viewport|AddtoViewport _output_get 0))))

(fn OpenFadeOut
  (Variables|Default|GetFadeOutRef
    (:then)
    (:else
      (bind _returnvalue (UserInterface|CreateWidget "/Game/KingOfRecess/Blueprints/UI/LoadingScreen/WG_FadeOutWg.WG_FadeOutWg_C"))
      (bind _output_get (Variables|Default|SetFadeOutRef _returnvalue))
      (UserInterface|Viewport|AddtoViewport _output_get 0))))