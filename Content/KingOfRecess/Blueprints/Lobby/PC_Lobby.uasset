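; PC_Lobby is the lobby player controller for King of Recess, relaying screen transition requests to the lobby HUD.
; Its events forward loading screen pop-ups, fade-ins and fade-outs to HUD_Lobby through GetHUDRef, which casts and caches the HUD on first use.
; A separate UpdateUI event, marked as not in use, initializes base UI on HUD_KOR instead.
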(event Custom|UpdateUI
  (params (UIClass :type User%20Widget%20Class%20Reference) (InputMode :type EInputMode%20Enum :default "UI"))
  ;[1 0.07247 0.05382] Not in use
  (bind _ashud_kor (Utilities|Casting|CastToHUD_KOR (HUD|GetHUD)))
  (Default|InitializeBaseUI _ashud_kor UIClass InputMode))

(event Custom|LoadPopUp
  (params (TutorialPopUp :type E_TutorialPopUp%20Enum :default "NewEnumerator0"))
  (Default|OpenLoadingScreen (CallFunction|GetHUDRef) TutorialPopUp))

(event Custom|FadeIn
  (Default|OpenFadein (CallFunction|GetHUDRef)))

(event Custom|FadeOut
  (Default|OpenFadeOut (CallFunction|GetHUDRef)))

(fn ConstructionScript)

(fn GetHUDRef
  (Variables|Default|GetHUDLobby
    (:then
      _)
    (:else
      (bind _ashud_lobby (Utilities|Casting|CastToHUD_Lobby (HUD|GetHUD)))
      (Variables|Default|SetHUDLobby _ashud_lobby)))
  (return (Variables|Default|GetHUDLobby)))