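; Manager for the Floor Is Lava minigame that runs timed rounds of rising and sinking platforms on the server.
; A looping timer raises Difficulty, sinks the current platforms, then after a delay asks PlatformSpawner for that difficulty's platform type.
; New platforms spawn at the center or random points of a configurable box and start floating.
; Once Difficulty exceeds MaxRounds, it tells the game mode's PhaseManager to activate the next phase.
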(event Custom|CreateRandomPlatforms
  (bind _platforms (Variables|Default|GetPlatforms))
  (bind _result (Math|Integer|IncrementInt (Variables|Default|GetDifficulty))
    (:%20%20
      (if (> _result (Variables|Default|GetMaxRounds))
        (Development|PrintString "GameFinished")
        (bind _askor_base_gm (Utilities|Casting|CastToKorBaseGM (Game|GetGameMode))
          (:then
            (Class|PhaseManager|ActivateNextPhase (Variables|/Script/KOR.KorBaseGM|GetPhaseManager _askor_base_gm) true))
          (:CastFailed
            (Utilities|String|LogString "ERROR, NOT GAME MODE FOUND")))
        (else
          (bind (_arrayindex _arrayelement) (Utilities|Array|ReverseforEachLoop _platforms)
            (:LoopBody
              (Default|Sink _arrayelement true)
              (Utilities|Array|RemoveIndex _platforms _arrayindex))
            (:Completed
              (Utilities|FlowControl|Delay 5.0)
              (Variables|Default|SetCurrentPlatform (Class|PlatformSpawner|GetPlatform (Variables|Default|GetPlatformSpawner) (Variables|Default|GetDifficulty)))
              (bind _spawnpoints (CallFunction|ChooseSpawnPoints 0 (.spawnposition (Variables|Default|GetCurrentPlatform))))
              (for _array_element _spawnpoints
                (Development|PrintString (Utilities|GetClassDisplayName (.platformclass (Variables|Default|GetCurrentPlatform))))
                (bind _returnvalue (Game|SpawnActorfromClass (.platformclass (Variables|Default|GetCurrentPlatform)) (Math|Transform|MakeTransform _array_element "0, 0, 0" "1.000000,1.000000,1.000000") "AlwaysSpawn" "MultiplyWithRoot" 0 0))
                (bind _asbp_base_platform_actor (Utilities|Casting|CastToBP_BasePlatformActor _returnvalue))
                (Utilities|Array|Add (Variables|Default|GetPlatforms) _asbp_base_platform_actor)
                (Default|StartFloat _asbp_base_platform_actor)))))))))

(event Custom|EventRandomPlatforms
  (params (Time :type Float%20%28single-precision%29))
  (Utilities|Time|SetTimerbyEvent (delegate Custom|CreateRandomPlatforms) Time true))

(event EventBeginPlay
  (if (Networking|IsServer)
    (CallFunction|CreateRandomPlatforms)
    (CallFunction|EventRandomPlatforms 3e+01)))

(fn ConstructionScript
  (Components|Box|SetBoxExtent (Variables|Default|GetBox) (Variables|Default|GetBoxExtend) true))

(fn ChooseSpawnPoints
  (params (NumOfSpawnPoints :type Integer) (Selection :type ESpawnPosition%20Enum :default "CENTER"))
  (switch Utilities|FlowControl|Switch|SwitchonESpawnPosition Selection
    (:CENTER
      (return (Utilities|Array|MakeArray (Transformation|GetWorldLocation (Variables|Default|GetBox)))))
    (:RANDOM
      (for _index (range 0 NumOfSpawnPoints)
        (Utilities|Array|Add (LocalVariables|GetSpawnPositions) (CallFunction|GetRandomPosition)))
      (return (LocalVariables|GetSpawnPositions)))))

(fn GetRandomPosition
  (bind _box (Variables|Default|GetBox))
  (bind _boxextent (Variables|/Script/Engine.BoxComponent|GetBoxExtent _box))
  (bind _returnvalue (* (.y _boxextent) 1.0))
  (bind _returnvalue_2 (* (.x _boxextent) 1.0))
  (return (+ (Transformation|GetWorldLocation _box) (Math|Vector|MakeVector (Math|Conversions|ToFloat(Integer) (Class|KismetMathLibrary|RandomInteger64inRange (Class|KismetMathLibrary|ToInt64(Float) (* _returnvalue_2 -1.0)) (Class|KismetMathLibrary|ToInt64(Float) _returnvalue_2))) (Math|Conversions|ToFloat(Integer) (Class|KismetMathLibrary|RandomInteger64inRange (Class|KismetMathLibrary|ToInt64(Float) (* _returnvalue -1.0)) (Class|KismetMathLibrary|ToInt64(Float) _returnvalue))) 0.0))))