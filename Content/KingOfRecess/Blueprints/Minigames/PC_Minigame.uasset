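; Player controller Blueprint for King of Recess minigames, standing in until the C++ version replicates correctly.
; A server event emits pawn noise, then a multicast event spawns fart VFX behind the pawn and plays a random fart sound; its local trigger is disconnected.
; Other events forward fades, tutorial pop-ups and the countdown menu to HUD_KOR through a lazily cached getter.
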(event Custom|PlayFartMulticast
  (params (PC :type Kor%20Base%20PC%20Object%20Reference) (ControlledPawn :type Pawn%20Object%20Reference))
  (bind _returnvalue (Transformation|GetActorForwardVector ControlledPawn))
  (bind _returnvalue_2 (Transformation|GetActorLocation ControlledPawn))
  (Niagara|SpawnSystematLocation "/Game/KingOfRecess/VFX/Farts/NS_Fart.NS_Fart" (- _returnvalue_2 (* _returnvalue "50.000000,50.000000,50.000000")) (Math|Rotator|MakeRotfromX (* _returnvalue -1.0)))
  (Audio|PlaySoundatLocation (.OutItem (Utilities|Array|Random (Variables|Default|GetFartSounds))) _returnvalue_2 "0, 0, 0" 1.0 1.0 0.0 0 0 PC 0))

(event Custom|PlayFartServer
  (params (PC :type Kor%20Base%20PC%20Object%20Reference) (Pawn :type Pawn%20Object%20Reference))
  (Class|Actor|MakeNoise PC 1.0 Pawn (Transformation|GetActorLocation Pawn) 0.0 "None")
  (CallFunction|PlayFartMulticast PC Pawn))

(event Custom|FadeOut
  (Default|FadeOut (CallFunction|GetHUDRef)))

(event Custom|LoadPopUp
  (params (TutorialPopUp :type E_TutorialPopUp%20Enum :default "NewEnumerator0"))
  (Default|OpenTransitionMenu (CallFunction|GetHUDRef) TutorialPopUp))

(event Custom|FadeIn
  (Default|Fadein (CallFunction|GetHUDRef)))

(event Custom|LoadCountdown
  (Default|OpenMiniGameMenu (CallFunction|GetHUDRef)))

(event Input|KeyboardEvents|F
  (params (Key :type Key%20Structure :default "None"))
  ;[1 0.2232 0] TODO: complete the C++ version (for now it does not replicate correctly so use this one)
)

(fn ConstructionScript)

(fn GetHUDRef
  (Variables|Default|GetHUDMinigame
    (:then
      _)
    (:else
      (bind _ashud_kor (Utilities|Casting|CastToHUD_KOR (HUD|GetHUD)))
      (Variables|Default|SetHUDMinigame _ashud_kor)))
  (return (Variables|Default|GetHUDMinigame)))