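; BP_ChangePlayerColor is a game phase that gives the first local player a random color.
; On activation it waits a second, rolls one of eight color indices, stores it on the KorBasePC player controller and applies it through SetPlayerColorMaterial, then ends the phase.
; Disconnected leftover nodes show an alternate approach that sets the character mesh material from the game mode's PlayerColors array and removes entries from it.
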(event EventOnPhaseActivated
  (bind _worldcontext (Variables|Default|GetWorldContext))
  (Utilities|FlowControl|Delay _worldcontext 1.0)
  (bind _askor_base_pc (Utilities|Casting|CastToKorBasePC (Game|GetPlayerController _worldcontext)))
  (bind _output_get (Variables|/Script/KOR.KorBasePC|SetPlayerColorIndex _askor_base_pc (Math|Random|RandomInteger 8)))
  (Class|KorBasePC|SetPlayerColorMaterial _askor_base_pc _output_get)
  (Class|Phase|PhaseEnd))