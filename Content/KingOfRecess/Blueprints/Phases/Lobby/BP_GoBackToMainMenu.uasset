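; Lobby phase Blueprint that returns the game from the lobby to the main menu.
; On activation it runs only on the server, where it calls a ChangeLevel event guarded by a DoOnce.
; That event opens the MainMenu level by object reference and then ends the phase.
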(event Custom|ChangeLevel
  (Utilities|FlowControl|DoOnce false
    (:Completed
      (Game|OpenLevel(byObjectReference) (Variables|Default|GetWorldContext) (Variables|/Script/KOR.KorGMDefinition|GetLevel (Variables|Default|GetMainMenu)))
      (Class|Phase|PhaseEnd))))

(event EventOnPhaseActivated
  (if (Networking|IsServer (Variables|Default|GetWorldContext))
    (CallFunction|ChangeLevel)))