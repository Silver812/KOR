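; Lobby phase Blueprint for King of Recess that holds until all players have been added.
; On activation it binds to the base game mode's player-joined and add-players-completed events, and finishes immediately if all players are already added.
; It also provides an event that opens a pop-up through a player's lobby controller, and a finish event that ends the phase.
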(event Custom|OpenPopUp_Client
  (params (PlayerController :type Player%20Controller%20Object%20Reference))
  (bind _aspc_lobby (Utilities|Casting|CastToPC_Lobby PlayerController))
  (Default|LoadPopUp _aspc_lobby "NewEnumerator1"))

(event Custom|FinishPhase
  (Class|Phase|PhaseEnd))

(event EventOnPhaseActivated
  (bind _askor_base_gm (Utilities|Casting|CastToKorBaseGM (Game|GetGameMode (Variables|Default|GetWorldContext))))
  (EventDispatchers|BindEventtoOnPlayerJoined _askor_base_gm (EventDispatchers|CreateEvent :!event Custom|OpenPopUp_Client))
  (EventDispatchers|BindEventtoOnAddPlayersCompleted _askor_base_gm (EventDispatchers|CreateEvent :!event Custom|FinishPhase))
  (if (Variables|/Script/KOR.KorBaseGM|GetbAllPlayersAdded _askor_base_gm)
    (CallFunction|FinishPhase)))