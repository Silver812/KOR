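; BP_WFAPLobbyScore is a lobby phase that holds the game flow until the game mode reports all players added.
; On activation it binds to KorBaseGM's player-joined and add-players-completed events, and finishes at once if all players are already added.
; Finishing waits a short fixed delay, marked as a placeholder for a delegate, then ends the phase.
; A separate event calls FadeOut on a given lobby player controller.
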(event Custom|FadeOut_Client
  (params (PlayerController :type Player%20Controller%20Object%20Reference))
  (bind _aspc_lobby (Utilities|Casting|CastToPC_Lobby PlayerController))
  (Default|FadeOut _aspc_lobby))

(event Custom|FinishPhase
  ;[1 0.2232 0] TODO: change this with a delegate
  (Utilities|FlowControl|Delay (Variables|Default|GetWorldContext) 2.0)
  (Class|Phase|PhaseEnd))

(event EventOnPhaseActivated
  (bind _askor_base_gm (Utilities|Casting|CastToKorBaseGM (Game|GetGameMode (Variables|Default|GetWorldContext))))
  (EventDispatchers|BindEventtoOnPlayerJoined _askor_base_gm (EventDispatchers|CreateEvent :!event Custom|FadeOut_Client))
  (EventDispatchers|BindEventtoOnAddPlayersCompleted _askor_base_gm (EventDispatchers|CreateEvent :!event Custom|FinishPhase))
  (if (Variables|/Script/KOR.KorBaseGM|GetbAllPlayersAdded _askor_base_gm)
    (CallFunction|FinishPhase)))