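; BP_GoBackToLobby is a phase that returns the game from a minigame to a lobby scene.
; On activation, it runs once and picks one of two LobbyPool entries based on whether the ScoreManager's minigame counter is above zero.
; It stores that definition in GI_Kor as "Lobby", has KorBaseGM switch to its level as a listen server, then ends the phase.
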(event Custom|ChangeLevel
  (Utilities|FlowControl|DoOnce false
    (:Completed
      (if (> (Class|ScoreManager|GetMinigameCounter (Subsystems|GetScoreManager (Game|GetPlayerController (Variables|Default|GetWorldContext)))) 0)
        (Variables|Default|SetSelectedLobby 0)
        (else
          (Variables|Default|SetSelectedLobby 1)))
      (bind _asgi_kor (Utilities|Casting|CastToGI_Kor (Game|GetGameInstance (Variables|Default|GetWorldContext))))
      (Class|KorGI|SetGMDefinition _asgi_kor "Lobby" (Utilities|Array|Get(acopy) (Variables|Default|GetLobbyPool) (Variables|Default|GetSelectedLobby)))
      (bind _askor_base_gm (Utilities|Casting|CastToKorBaseGM (Game|GetGameMode (Variables|Default|GetWorldContext))))
      (Class|KorBaseGM|ChangetoNewSceneServerListen _askor_base_gm (Variables|/Script/KOR.KorGMDefinition|GetLevel (Utilities|Array|Get(acopy) (Variables|Default|GetLobbyPool) (Variables|Default|GetSelectedLobby))))
      (Class|Phase|PhaseEnd))))

(event EventOnPhaseActivated
  (CallFunction|ChangeLevel))