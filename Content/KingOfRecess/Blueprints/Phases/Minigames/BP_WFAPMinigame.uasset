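; Minigame phase that waits for all players to be added before the game moves on.
; On activation it binds to the base game mode's player-joined and add-players-completed events, and finishes directly if everyone is already added.
; A client popup event disables the player's input and loads a popup through the minigame player controller.
; Finishing holds for a fixed delay before ending the phase.
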(event Custom|OpenPopUp_Client
  (params (PlayerController :type Player%20Controller%20Object%20Reference))
  (Input|DisableInput PlayerController PlayerController)
  (bind _aspc_minigame (Utilities|Casting|CastToPC_Minigame PlayerController))
  (Default|LoadPopUp _aspc_minigame "NewEnumerator2"))

(event Custom|FinishPhase
  (Utilities|FlowControl|Delay (Variables|Default|GetWorldContext) 12.0)
  (Class|Phase|PhaseEnd))

(event EventOnPhaseActivated
  (bind _askor_base_gm (Utilities|Casting|CastToKorBaseGM (Game|GetGameMode (Variables|Default|GetWorldContext))))
  (EventDispatchers|BindEventtoOnPlayerJoined _askor_base_gm (EventDispatchers|CreateEvent :!event Custom|OpenPopUp_Client))
  (EventDispatchers|BindEventtoOnAddPlayersCompleted _askor_base_gm (EventDispatchers|CreateEvent :!event Custom|FinishPhase))
  (if (Variables|/Script/KOR.KorBaseGM|GetbAllPlayersAdded _askor_base_gm)
    (CallFunction|FinishPhase)))